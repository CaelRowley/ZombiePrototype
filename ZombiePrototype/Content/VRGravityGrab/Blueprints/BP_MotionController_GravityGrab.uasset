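; VR motion controller hand that pulls pickup objects from a distance into the player's grasp with gravity grab.
; Each tick a fingertip sphere trace outlines a target, which the grab launches along a distance-scaled projectile arc with briefly boosted mass.
; An enlarged grab sphere triggers slow motion and glove glow as the object arrives.
; It also builds per-bone sphere hand collision and offsets the hand mesh per headset.
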(event OnComponentBeginOverlap(GrabSphere)
  (params (OverlappedComponent :type Primitive%20Component%20Object%20Reference) (OtherActor :type Actor%20Object%20Reference) (OtherComp :type Primitive%20Component%20Object%20Reference) (OtherBodyIndex :type Integer) (bFromSweep :type Boolean) (SweepResult :type Hit%20Result%20Structure%20%28by%20ref%29))
  ;[1 0.25 0] When The Gravity Grabbed Object Touchs The Grab Sphere, Start Slow Motion.
  (if (and (Variables|Default|GetPeformingGravityGrab) (== OtherActor (Variables|Default|GetGravityGrabActor)))
    (Utilities|Time|SetGlobalTimeDilation 0.1)
    (Rendering|Material|SetScalarParameterValue (Variables|Default|GetMaterial) "Glow" 1.0 :!class /Script/Engine.MaterialInstanceDynamic)))

(event OnComponentEndOverlap(GrabSphere)
  (params (OverlappedComponent :type Primitive%20Component%20Object%20Reference) (OtherActor :type Actor%20Object%20Reference) (OtherComp :type Primitive%20Component%20Object%20Reference) (OtherBodyIndex :type Integer))
  ;[1 0.25 0] When The Gravity Grabbed Object Leaves The Grab Sphere, End Slow Motion.
  (if (and (Variables|Default|GetPeformingGravityGrab) (== OtherActor (Variables|Default|GetGravityGrabActor)))
    (Utilities|Time|SetGlobalTimeDilation 1.0)
    (Variables|Default|SetPeformingGravityGrab false)
    (Rendering|Material|SetScalarParameterValue (Variables|Default|GetMaterial) "Glow" 0.0 :!class /Script/Engine.MaterialInstanceDynamic)))

(event OnActorHit(GravityGrabActor)
  (params (SelfActor :type Actor%20Object%20Reference) (OtherActor :type Actor%20Object%20Reference) (NormalImpulse :type Vector :default "0, 0, 0") (Hit :type Hit%20Result%20Structure%20%28by%20ref%29))
  (Utilities|Casting|CastToBP_MotionController_GravityGrab OtherActor
    (:CastFailed
      (Class|PickupOutlineInterface|ToggleOutline(Message) (Variables|Default|GetGravityGrabActor) false)
      (Variables|Default|SetPeformingGravityGrab false)
      (Development|PrintString "Gravity Out"))))

(event OnDestroyed(GravityGrabActor)
  (params (DestroyedActor :type Actor%20Object%20Reference))
  (Variables|Default|SetPeformingGravityGrab false)
  (Development|PrintString "Gravity Out"))

(event Custom|Do%20Gravity%20Grab
  (bind _gravitygrabactor (Variables|Default|GetGravityGrabActor))
  (bind _gravitygrabactor_2 (Variables|Default|GetGravityGrabActor))
  (bind _returnvalue (Actor|GetComponentbyClass _gravitygrabactor_2 "/Script/Engine.PrimitiveComponent"))
  ;[1 0.25 0] When Player Press Trigger, Check If We Have A Grab Target To Start Gravity Grab.
  (if (Variables|Default|GetHasGravityGrabTarget)
    (Variables|Default|SetPeformingGravityGrab true)
    ;[1 0.25 0] Enlarge Grab Sphere To Make Grabbing Easier
    (Components|Sphere|SetSphereRadius (Variables|Default|GetGrabSphere) (Variables|Default|GetGrabSphereRadius_GravityGrab) true)
    ;[1 0.25 0] Calculate Velocity That Can Fly The Grabbed Object To The Hand
    (Utilities|IsValid _gravitygrabactor
      (:Is%20Valid
        (bind _launchvelocity (CallFunction|TraceGravityGrabPath _gravitygrabactor (Transformation|GetSocketLocation (Variables|Default|GetHandMesh) (Variables|Default|GetTraceStartSocketName))))
        ;[1 0.25 0] Apply Velocity To Make Grabbed Object Fly.
        (Utilities|IsValid _returnvalue
          (:Is%20Valid
            (bind _output_get (Variables|Default|SetGravityGrabPrimitive _returnvalue))
            (Class|PrimitiveComponent|SetAllPhysicsLinearVelocity _output_get _launchvelocity false)
            (Class|PrimitiveComponent|SetLinearDamping (Variables|Default|GetGravityGrabPrimitive) 0.0)
            ;[1 0.25 0] Increase Flying Object's Mass So It Won't  Be Blocked By Other Dynamic Objects. ( Will Push Them Away )
            (Class|PrimitiveComponent|SetMassScale (Variables|Default|GetGravityGrabPrimitive) "None" 1e+04)
            (Utilities|FlowControl|Delay 0.2)
            (Utilities|IsValid (Variables|Default|GetGravityGrabPrimitive)
              (:Is%20Valid
                (Class|PrimitiveComponent|SetMassScale (Variables|Default|GetGravityGrabPrimitive) "None" 1.0)))))))))

(event EventBeginPlay
  (|CallParentFunction)
  ;[1 0.25 0] Create Dynamic Material So Glowing Effect Can Be Turn On / Off
  (bind _returnvalue (Rendering|Material|CreateDynamicMaterialInstance (Variables|Default|GetHandMesh) 0 (Rendering|Material|GetMaterial (Variables|Default|GetHandMesh) 0) "None" :!class /Script/Engine.PrimitiveComponent))
  (Variables|Default|SetMaterial _returnvalue)
  ;[1 0.25 0] Creat Collision On Hand Mesh, Delay To Wait Before MotionControllerPawn Finishs Initializing.
  (Utilities|FlowControl|Delay 1.0)
  (CallFunction|SetupHandCollision))

(event EventTick
  (params (DeltaSeconds :type Float%20%28single-precision%29))
  ;[1 0.25 0] Check For Objects That Can Be Gravity Grabbed.
  (CallFunction|CheckGravityGrab)
  (|CallParentFunction DeltaSeconds))

(fn ConstructionScript
  ;[1 0.25 0] Set Trace Socket Name By Hand
  (|CallParentFunction)
  (Variables|Default|SetTraceStartSocketName (Utilities|Select :Index (Variables|Default|GetHand) :Left "indexSocket" :Right "indexSocket" :AnyHand "None" :Pad "None" :ExternalCamera "None" :Gun "None" :Special_1 "None" :Special_2 "None" :Special_3 "None" :Special_4 "None" :Special_5 "None" :Special_6 "None" :Special_7 "None" :Special_8 "None" :Special_9 "None" :Special_10 "None" :Special_11 "None")))

(fn CheckGravityGrab
  (bind _handmesh (Variables|Default|GetHandMesh))
  (bind _tracestartsocketname (Variables|Default|GetTraceStartSocketName))
  (bind _returnvalue (Transformation|GetSocketTransform _handmesh _tracestartsocketname "RTS_World"))
  (bind (_location _rotation) (Math|Transform|BreakTransform _returnvalue))
  (if (Variables|Default|GetPeformingGravityGrab)
    (Utilities|IsValid (Variables|Default|GetGravityGrabActor)
      (:Is%20Valid
        ;[1 0.25 0] Check Velocity of Gravity Grabbed Actor
        (if (< (Math|Vector|VectorLengthSquared (Transformation|GetVelocity (Variables|Default|GetGravityGrabActor))) 1e+02)
          ;[1 0.25 0] If Gravity Grabbed Actor Has Slow Down For A While, End Gravity Grab
          (bind _output_get (Variables|Default|SetGravityGrabExitTimer (+ (Variables|Default|GetGravityGrabExitTimer) (Utilities|Time|GetWorldDeltaSeconds))))
          (if (> _output_get (Variables|Default|GetGravityGrabExitTime))
            (Class|PickupOutlineInterface|ToggleOutline(Message) (Variables|Default|GetGravityGrabActor) false)
            (Variables|Default|SetPeformingGravityGrab false)
            (Variables|Default|SetGravityGrabActor 0)
            (Variables|Default|SetGravityGrabExitTimer 0.0))
          (else
            (Variables|Default|SetGravityGrabExitTimer 0.0))))
      (:Is%20Not%20Valid
        ;[1 0.25 0] If GravityGrabActor is Not Valid, End Gravity Grab
        (Variables|Default|SetPeformingGravityGrab false)
        (Variables|Default|SetGravityGrabExitTimer 0.0)))
    (else
      ;[1 0.25 0] Trace For Objects That Can Be Gravity Grabbed.
      (bind (_outhit _returnvalue_2) (Collision|SphereTraceForObjects _location (+ _location (* (Math|Vector|GetForwardVector _rotation) (Variables|Default|GetGravityGrabRange))) 2.0 (Utilities|Array|MakeArray "ObjectTypeQuery2" "ObjectTypeQuery4" "ObjectTypeQuery3" "ObjectTypeQuery5" "ObjectTypeQuery6") true 0 "None"))
      (if _returnvalue_2
        ;[1 0.25 0] Only Pickable Objects Can Be Grabbed.
        (if (Utilities|DoesObjectImplementInterface (.HitActor (Collision|BreakHitResult _outhit)) "/Game/VRGravityGrab/VRTemplate/Blueprints/PickupActorInterface.PickupActorInterface_C")
          ;[1 0.25 0] If Grabbable Object Is Found, Store It In "Gravity Grab Actor" Variable.
          (Utilities|IsValid (Variables|Default|GetGravityGrabActor)
            (:Is%20Valid
              (Class|PickupOutlineInterface|ToggleOutline(Message) (Variables|Default|GetGravityGrabActor) false))
            (:Is%20Not%20Valid
              _))
          (bind _output_get_2 (Variables|Default|SetGravityGrabActor (.HitActor (Collision|BreakHitResult _outhit))))
          ;[1 0.25 0] If Gravity Grab Target Is Already Grabbed, Stop Gravity Grab. Else Highlight The Grab Target.
          (Utilities|IsValid (Variables|Default|GetAttachedActor)
            (:Is%20Valid
              (Class|PickupOutlineInterface|ToggleOutline(Message) _output_get_2 (select (== (Variables|Default|GetAttachedActor) (Variables|Default|GetGravityGrabActor)) false true))
              (bind _output_get_3 (Variables|Default|SetHasGravityGrabTarget (select (== (Variables|Default|GetAttachedActor) (Variables|Default|GetGravityGrabActor)) false true)))
              (Variables|Default|SetPeformingGravityGrab _output_get_3)
              (Variables|Default|SetGravityGrabActor 0))
            (:Is%20Not%20Valid
              (Variables|Default|SetHasGravityGrabTarget true)
              (Class|PickupOutlineInterface|ToggleOutline(Message) (Variables|Default|GetGravityGrabActor) true)))
          (else
            ;[1 0.25 0] No Grabbable Object Found. Abort Gravity Grab.
            (Variables|Default|SetHasGravityGrabTarget false :!label _label)
            (Utilities|IsValid (Variables|Default|GetGravityGrabActor)
              (:Is%20Valid
                (Class|PickupOutlineInterface|ToggleOutline(Message) (Variables|Default|GetGravityGrabActor) false)
                (Variables|Default|SetGravityGrabActor 0)))))
        (else
          (goto _label))))))

(fn TraceGravityGrabPath
  (params (GrabbedActor :type Actor%20Object%20Reference) (HandLocation :type Vector))
  (bind _returnvalue (Transformation|GetActorLocation GrabbedActor))
  (Utilities|IsValid GrabbedActor
    (:Is%20Valid
      ;[1 0.25 0] Calculate Flying Velocity.
      (bind _outlaunchvelocity (Game|SuggestProjectileVelocityCustomArc _returnvalue HandLocation 0.0 (Math|Float|Lerp 0.4 0.9 (Math|Float|Clamp(Float) (/ (Math|Vector|Distance(Vector) _returnvalue HandLocation) (Variables|Default|GetGravityGrabRange))))))
      (return _outlaunchvelocity))
    (:Is%20Not%20Valid
      (return "0, 0, 0"))))

(fn GrabActor
  (|CallParentFunction)
  ;[1 0.25 0] Finish Grabbing, Reset Grab Sphere Radius To Normal.
  (Components|Sphere|SetSphereRadius (Variables|Default|GetGrabSphere) (Variables|Default|GetGrabSphereRadius_Normal) true)
  ;[1 0.25 0] After We Did Gravity Grab, Stop Slow Motion And Turn Off Glove Glowing Effect.
  (if (Variables|Default|GetPeformingGravityGrab)
    (Utilities|Time|SetGlobalTimeDilation 1.0)
    (Variables|Default|SetPeformingGravityGrab false)
    (Rendering|Material|SetScalarParameterValue (Variables|Default|GetMaterial) "Glow" 0.0 :!class /Script/Engine.MaterialInstanceDynamic)))

(fn SetupHandCollision
  ;[1 0.25 0] Attach One Sphere Collision To Each Bone Of The Hand Mesh. To Make Precise Physics Collision For Hand And Finger.
  (for _array_element (Transformation|GetAllSocketNames (Variables|Default|GetHandMesh))
    (if (Utilities|String|EndsWith (Utilities|String|ToString(Name) _array_element) "_r")
      (bind _returnvalue (AddComponent|AddSphereComponent true))
      (Collision|SetCollisionResponsetoAllChannels _returnvalue "ECR_Block")
      (Physics|SetSimulatePhysics _returnvalue false)
      (Collision|SetCollisionEnabled _returnvalue "PhysicsOnly")
      (Components|Sphere|SetSphereRadius _returnvalue 1.0 true)
      (Transformation|AttachComponentToComponent _returnvalue (Variables|Default|GetHandMesh) _array_element "SnapToTarget" "SnapToTarget" "KeepWorld" false))))

(fn SetupGravityGrabPointer
  (Transformation|AttachComponentToComponent (Variables|Default|GetGravityGrabPointer) (Variables|Default|GetHandMesh) (Variables|Default|GetTraceStartSocketName) "SnapToTarget" "SnapToTarget" "KeepWorld" true))

(fn SetupHandMeshbyDevice
  (params (HMDDevice%20Name :type Name))
  (switch name HMDDevice%20Name
    (:Default
      ;[1 0.25 0] Hand Mesh Offset For SteamVR Controllers ( Index and Vive )
      (LocalVariables|SetRelativeLocation "0, 0, 0" :!label _label)
      (LocalVariables|SetRelativeRotation "0, 0, 0")
      (LocalVariables|SetRelativeScale (select (Utilities|Enum|Equal(Enum) (Variables|Default|GetHand) "Left") "1.000000,-1.000000,1.000000" "1.000000,1.000000,1.000000")))
    (:OculusHMD
      ;[1 0.25 0] Hand Mesh Offset For Oculus Touch Controller
      (LocalVariables|SetRelativeLocation "-12.785664,-0.028015,-1.789026")
      (LocalVariables|SetRelativeRotation "0, 0,90.000000")
      (LocalVariables|SetRelativeScale (select (Utilities|Enum|Equal(Enum) (Variables|Default|GetHand) "Left") "1.000000,1.000000,-1.000000" "1.000000,1.000000,1.000000")))
    (:SteamVR
      (goto _label))
    (:PSVR
      (goto _label)))
  (Transformation|SetRelativeTransform (Variables|Default|GetHandMesh) (Math|Transform|MakeTransform (LocalVariables|GetRelativeLocation) (LocalVariables|GetRelativeRotation) (LocalVariables|GetRelativeScale)) false false))