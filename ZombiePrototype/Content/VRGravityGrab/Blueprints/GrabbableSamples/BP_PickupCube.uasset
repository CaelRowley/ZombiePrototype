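; BP_PickupCube is a sample VR grabbable cube for the gravity grab system.
; A dynamic material created at BeginPlay drives a Glow parameter that toggles the outline when the cube is targeted.
; Pickup disables physics and snaps the cube to the hand mesh's cubeSocket, while Drop re-enables physics and detaches it.
; SetGripType returns a fixed grip enum value for this object.
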(event EventBeginPlay
  (bind _cube (Variables|Default|GetCube))
  ;[1 0.25 0] Create Dynamic Material Instance So Outline Glowing Can Be Turn On / Off.
  (bind _returnvalue (Rendering|Material|CreateDynamicMaterialInstance _cube 0 (Rendering|Material|GetMaterial _cube 0) "None" :!class /Script/Engine.PrimitiveComponent))
  (Variables|Default|SetMaterial _returnvalue))

(event EventPickup
  (params (AttachTo :type Scene%20Component%20Object%20Reference) (HandMesh :type Scene%20Component%20Object%20Reference) (HandType :type EControllerHand%20Enum :default "Left") (FlipSocket :type Boolean))
  (Physics|SetSimulatePhysics (Variables|Default|GetCube) false)
  (Transformation|AttachComponentToComponent (VehicleSound|GetRootComponent) HandMesh "cubeSocket" "SnapToTarget" "SnapToTarget" "KeepWorld" false))

(event EventDrop
  (Physics|SetSimulatePhysics (Variables|Default|GetCube) true)
  (Transformation|DetachFromActor "KeepWorld" "KeepWorld" "KeepWorld"))

(event EventToggleOutline
  (params (ShowOutline :type Boolean))
  ;[1 0.25 0] When Become Grab Target, Show Outline
  (Rendering|Material|SetScalarParameterValue (Variables|Default|GetMaterial) "Glow" (select ShowOutline 1.0 0.0) :!class /Script/Engine.MaterialInstanceDynamic))

(fn ConstructionScript)

(fn SetGripType
  (return "NewEnumerator4"))